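; Blueprint function library of helpers for a settings menu that works with graphics quality options.
; GetSldiers gathers the children of a slider container that implement BPI_Slider.
; GetSettingsValues reads the scalability quality levels, from view distance to shading, from GameUserSettings.
; GetSettingsValuesAsArray repacks those levels into a fixed-order array.
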(fn `GetSettingsValues`
  (returns (ViewDistance :type Integer) (AntiAliasing :type Integer) (PostProcessing :type Integer) (Shadows :type Integer) (Textures :type Integer) (VisualEffects :type Integer) (Foliage :type Integer) (Shading :type Integer))
  (bind _returnvalue (`GameUserSettings.GetGameUserSettings`))
  (return (`GameUserSettings.GetViewDistanceQuality` _returnvalue) (`GameUserSettings.GetAntiAliasingQuality` _returnvalue) (`GameUserSettings.GetPostProcessingQuality` _returnvalue) (`GameUserSettings.GetShadowQuality` _returnvalue) (`GameUserSettings.GetTextureQuality` _returnvalue) (`GameUserSettings.GetVisualEffectQuality` _returnvalue) (`GameUserSettings.GetFoliageQuality` _returnvalue) (`GameUserSettings.GetShadingQuality` _returnvalue)))

(fn `GetSettingsValuesAsArray`
  (returns (Values :type "Array of Integer"))
  (bind (_viewdistance _antialiasing _postprocessing _shadows _textures _visualeffects _foliage _shading) (`self.GetSettingsValues` (`local.__WorldContext`)))
  (return (`|MakeArray` _viewdistance _antialiasing _postprocessing _shadows _textures _visualeffects _foliage _shading)))

(fn `GetSldiers`
  (params (SlidersContainer :type "PanelWidget Object Reference"))
  (returns (ContainedSliders :type "Array of Widget Object Reference"))
  (locals (CurrentChild :type "Widget Object Reference") (Sliders :type "Array of Widget Object Reference"))
  (for _index (range (`PanelWidget.GetChildrenCount` SlidersContainer))
    (bind _output_get (set `local.CurrentChild` (`PanelWidget.GetChildAt` (`local.SlidersContainer`) _index)))
    (if (`KismetSystemLibrary.DoesImplementInterface` _output_get "/SettingsPack/Blueprints/Interfaces/BPI_Slider.BPI_Slider_C")
      (`KismetArrayLibrary.Array_Add` (`local.Sliders`) (`local.CurrentChild`))))
  (return (`local.Sliders`)))